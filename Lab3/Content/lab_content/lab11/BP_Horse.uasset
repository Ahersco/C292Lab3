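; BP_Horse is a child animal Blueprint from a lab exercise that, despite its name, labels itself a crow with a "caww" sound.
; BeginPlay sets the inherited-style Animal and Sound values, and Tick reassigns MoveSpeed every frame, each before calling the parent implementation.
; Overlap with the first-person character only calls Activate on the root scene component, without calling the parent.
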(event EventBeginPlay
  (Variables|Default|SetAnimal " crow ")
  (Variables|Default|SetSound " caww")
  (|CallParentFunction))

(event Collision|EventActorBeginOverlap
  (params (OtherActor :type Actor%20Object%20Reference))
  (Utilities|Casting|CastToBP_FirstPersonCharacter OtherActor)
  (Components|Activation|Activate (Variables|Default|GetDefaultSceneRoot) false))

(event EventTick
  (params (DeltaSeconds :type Float%20%28single-precision%29))
  (Variables|Default|SetMove%20Speed 3.0)
  (|CallParentFunction DeltaSeconds))

(fn ConstructionScript
  (|CallParentFunction))