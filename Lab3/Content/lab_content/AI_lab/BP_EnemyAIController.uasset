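; AI controller for an enemy pawn that patrols points and chases what it perceives.
; After a short delay on BeginPlay, it casts its pawn to BP_EnemyAIPawn and loops AIMoveTo through that pawn's patrol points, advancing on success or failure.
; A successful AIPerception stimulus stores the actor as target, stops movement and moves toward it.
; Losing the stimulus clears the target and resumes patrol.
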(event OnTargetPerceptionUpdated(AIPerception)
  (params (Actor :type Actor%20Object%20Reference) (Stimulus :type AI%20Stimulus%20Structure))
  (Development|PrintString "sees")
  (if (.bSuccessfullySensed (Utilities|Struct|BreakAIStimulus Stimulus))
    (bind _output_get (Variables|Default|Settarget%20actor Actor))
    (AI|Navigation|StopMovement)
    (AI|AIMoveTo (Variables|Default|GetPawn%20ref) "0, 0, 0" _output_get 5.0 false)
    (else
      (Variables|Default|Settarget%20actor 0)
      (CallFunction|Patrol))))

(event Custom|Patrol
  (bind _pawn_ref (Variables|Default|GetPawn%20ref))
  (AI|AIMoveTo (Variables|Default|GetPawn%20ref) (Transformation|GetActorLocation (Utilities|Array|Get(acopy) (Variables|/Game/lab_content/AI_lab/BP_EnemyAIPawn.BP_EnemyAIPawn_C|GetPatrol%20Points _pawn_ref) (Variables|/Game/lab_content/AI_lab/BP_EnemyAIPawn.BP_EnemyAIPawn_C|Getcurrent%20partol%20index _pawn_ref))) 0 5.0 false
    (:OnSuccess
      _)
    (:OnFail
      _))
  (Default|GetNextPatrolPoint (Variables|Default|GetPawn%20ref))
  (CallFunction|Patrol))

(event EventBeginPlay
  (Utilities|FlowControl|Delay 0.5)
  (bind _asbp_enemy_aipawn (Utilities|Casting|CastToBP_EnemyAIPawn (Pawn|GetControlledPawn)))
  (Variables|Default|SetPawn%20ref _asbp_enemy_aipawn)
  (CallFunction|Patrol))

(fn ConstructionScript)