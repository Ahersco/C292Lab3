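; BP_AICharacter is an enemy that chases the player and resolves contact based on whether the player carries a knife.
; Tick reissues an AI move toward the player capsule's location every frame.
; On overlap with BP_FirstPersonCharacter, a knife holder kills it, spawning a BP_Key at its transform before it is destroyed.
; Without a knife, it only prints a GameOver message.
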(event Collision|EventActorBeginOverlap
  (params (OtherActor :type Actor%20Object%20Reference))
  (bind _asbp_first_person_character (Utilities|Casting|CastToBP_FirstPersonCharacter OtherActor))
  (if (Variables|/Game/FirstPerson/Blueprints/BP_FirstPersonCharacter.BP_FirstPersonCharacter_C|GetHas%20Knife _asbp_first_person_character)
    (Game|SpawnActorfromClass "/Game/lab_content/lab16/BP_Key.BP_Key_C" (Transformation|GetActorTransform self) "Undefined" "MultiplyWithRoot" 0 0)
    (Development|PrintString "dead")
    (Actor|DestroyActor self)
    (else
      (Development|PrintString "GameOver"))))

(event EventTick
  (params (DeltaSeconds :type Float%20%28single-precision%29))
  (AI|AIMoveTo self (Transformation|GetWorldLocation (Variables|/Script/Engine.Character|GetCapsuleComponent (Game|GetPlayerCharacter 0))) 0 5.0 false))

(fn ConstructionScript)