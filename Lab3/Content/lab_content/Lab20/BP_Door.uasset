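; BP_Door is a lab door actor that reacts to left and right BP_Button presses with a debug message.
; On BeginPlay it finds the first button tagged for each side and binds DoorOpen to that button's matching right or left press dispatcher.
; Both dispatchers call the same event, which prints the side from the door's own IsRight flag, whichever button fired, and does not move the door.
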(event Custom|Door%20Open
  (if (Variables|Default|Getis%20Right)
    (Development|PrintString "Door right" true true "(R=0.000000,G=0.660000,B=1.000000,A=1.000000)" 3e+01)
    (else
      (Development|PrintString "door left" true true "(R=0.000000,G=0.660000,B=1.000000,A=1.000000)" 3e+01))))

(event EventBeginPlay
  (bind _outactors (Actor|GetAllActorsOfClasswithTag "/Game/lab_content/Lab20/BP_Button.BP_Button_C" "Right_Button"))
  (EventDispatchers|BindEventtoOnButtonPressRight (Utilities|Array|Get(acopy) _outactors) (delegate Custom|Door%20Open))
  (bind _outactors_2 (Actor|GetAllActorsOfClasswithTag "/Game/lab_content/Lab20/BP_Button.BP_Button_C" "Left_Button"))
  (EventDispatchers|BindEventtoOnButtonPressLeft (Utilities|Array|Get(acopy) _outactors_2) (delegate Custom|Door%20Open)))

(fn ConstructionScript)