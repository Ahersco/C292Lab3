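; BP_Hatch is a hatch that reacts to button presses, currently only printing a debug message instead of opening.
; On BeginPlay it finds the first BP_Button tagged Right_Button and the first tagged Left_Button, binding HatchOpen to their respective right and left press dispatchers.
; Either press fires the same event, whose right or left message depends on the hatch's IsRight flag, not on which button fired.
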(event Custom|Hatch%20open
  (if (Variables|Default|Getis%20right)
    (Development|PrintString "hactch right")
    (else
      (Development|PrintString "hatcj left"))))

(event EventBeginPlay
  (bind _outactors (Actor|GetAllActorsOfClasswithTag "/Game/lab_content/Lab20/BP_Button.BP_Button_C" "Right_Button"))
  (EventDispatchers|BindEventtoOnButtonPressRight (Utilities|Array|Get(acopy) _outactors) (delegate Custom|Hatch%20open))
  (bind _outactors_2 (Actor|GetAllActorsOfClasswithTag "/Game/lab_content/Lab20/BP_Button.BP_Button_C" "Left_Button"))
  (EventDispatchers|BindEventtoOnButtonPressLeft (Utilities|Array|Get(acopy) _outactors_2) (delegate Custom|Hatch%20open)))

(fn ConstructionScript)