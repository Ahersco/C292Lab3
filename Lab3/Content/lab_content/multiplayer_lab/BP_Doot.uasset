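; BP_Doot is a door actor in the multiplayer lab that swings on interaction.
; Interact toggles the replicated IsOpen variable, whose RepNotify calls the open or close event.
; Those events play or reverse the OpenClose timeline, whose alpha drives relative yaw through a 90-degree swing.
; The RepNotify mapping is inverted: IsOpen true calls CloseDoor and false calls OpenDoor.
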(event Custom|open%20door
  (bind _open_alpha (Timeline|open%20close Play)
    (:Update
      (Transformation|SetActorRelativeRotation (Math|Rotator|MakeRotator 0.0 0.0 (* _open_alpha 9e+01))))))

(event Custom|close%20door
  (bind _open_alpha (Timeline|open%20close Reverse)
    (:Update
      (Transformation|SetActorRelativeRotation (Math|Rotator|MakeRotator 0.0 0.0 (* _open_alpha 9e+01))))))

(event EventBeginPlay)

(event Collision|EventActorBeginOverlap
  (params (OtherActor :type Actor%20Object%20Reference)))

(event EventTick
  (params (DeltaSeconds :type Float%20%28single-precision%29)))

(event EventInteract
  (Variables|Default|Setis%20open (not (Variables|Default|Getis%20open))))

(fn ConstructionScript)

(fn OnRepIsOpen
  (if (Variables|Default|Getis%20open)
    (CallFunction|CloseDoor)
    (else
      (CallFunction|OpenDoor))))