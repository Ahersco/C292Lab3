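; BP_Animal is an animal Blueprint that announces its sound on begin play and is meant to move.
; MakeSound prints a message built from the Animal and Sound variables.
; Tick calls Move every frame to play a timeline, but the location update is never executed.
; That disconnected node would lerp from the current location toward a world X position set by MoveSpeed, using the timeline's track as alpha.
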(event Custom|Make%20Sound
  (Development|PrintString (Utilities|String|Append (Variables|Default|GetAnimal) "Says" (Variables|Default|GetSound))))

(event Custom|Move
  (bind _newtrack_1 (Timeline|Timeline Play)))

(event EventBeginPlay
  (CallFunction|MakeSound))

(event EventTick
  (params (DeltaSeconds :type Float%20%28single-precision%29))
  (CallFunction|Move))

(fn ConstructionScript)