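; BP_GameState handles saving and loading of player health, transform and chest contents through a BP_GameSave object in the "DemoSave" slot.
; SaveGame writes its stored HP and transform variables, plus the first BP_Chest's contents, into a new save object.
; LoadGame restores those variables and that chest if the slot exists, then moves the first-person character to the saved transform.
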(event Custom|Save%20Game
  (bind _returnvalue (SaveGame|CreateSaveGameObject "/Game/Lab18/BP_GameSave.BP_GameSave_C"))
  (bind _output_get (Variables|Default|SetSave%20File _returnvalue))
  (Variables|/Game/Lab18/BP_GameSave.BP_GameSave_C|SetPlayer%20Health _output_get (Variables|Default|GetMax%20HP))
  (Variables|/Game/Lab18/BP_GameSave.BP_GameSave_C|SetPlayer%20Current%20HP _output_get (Variables|Default|GetCurrent%20HP))
  (Variables|/Game/Lab18/BP_GameSave.BP_GameSave_C|SetPlayer%20Transform _output_get (Variables|Default|GetPlayer%20Transform))
  (bind _outactors (Actor|GetAllActorsOfClass "/Game/Lab18/BP_Chest.BP_Chest_C"))
  (Variables|/Game/Lab18/BP_GameSave.BP_GameSave_C|SetChest%20Contents (Variables|Default|GetSave%20File) (Variables|/Game/Lab18/BP_Chest.BP_Chest_C|GetContents (Utilities|Array|Get(acopy) _outactors)))
  (SaveGame|SaveGametoSlot (Variables|Default|GetSave%20File) "DemoSave")
  (Development|PrintString "Game Saved"))

(event Custom|Load%20Game
  (bind _returnvalue (SaveGame|DoesSaveGameExist "DemoSave"))
  (if _returnvalue
    (bind _returnvalue_2 (SaveGame|LoadGamefromSlot "DemoSave"))
    (bind _asbp_game_save (Utilities|Casting|CastToBP_GameSave _returnvalue_2))
    (Development|PrintString "check")
    (bind _output_get (Variables|Default|SetSave%20File _asbp_game_save))
    (Variables|Default|SetCurrent%20HP (Variables|/Game/Lab18/BP_GameSave.BP_GameSave_C|GetPlayer%20Current%20HP _output_get))
    (Variables|Default|SetMax%20HP (Variables|/Game/Lab18/BP_GameSave.BP_GameSave_C|GetPlayer%20Health _output_get))
    (Variables|Default|SetPlayer%20Transform (Variables|/Game/Lab18/BP_GameSave.BP_GameSave_C|GetPlayer%20Transform _output_get))
    (bind _outactors (Actor|GetAllActorsOfClass "/Game/Lab18/BP_Chest.BP_Chest_C"))
    (Variables|/Game/Lab18/BP_Chest.BP_Chest_C|SetContents (Utilities|Array|Get(acopy) _outactors) (Variables|/Game/Lab18/BP_GameSave.BP_GameSave_C|GetChest%20Contents (Variables|Default|GetSave%20File)))
    (bind _asbp_first_person_character (Utilities|Casting|CastToBP_FirstPersonCharacter (Game|GetPlayerCharacter 0)))
    (Development|PrintString "check")
    (Transformation|SetActorTransform _asbp_first_person_character (Variables|Default|GetPlayer%20Transform))
    (else
      (Development|PrintString "slot not found"))))