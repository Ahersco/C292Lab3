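; BP_Platform is an interactive platform that the first-person character can raise with the F key once its ConeCollected flag is set.
; Overlap with that character stores the reference and enables input on the actor, with no matching disable.
; F plays a timeline that lerps the Cube from its current location toward a fixed world position, compounding each update.
; Without the cone, it prints a "can't move" message.
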(event Collision|EventActorBeginOverlap
  (params (OtherActor :type Actor%20Object%20Reference))
  (bind _asbp_first_person_character (Utilities|Casting|CastToBP_FirstPersonCharacter OtherActor))
  (Input|EnableInput (Game|GetPlayerController 0)))

(event Input|KeyboardEvents|F
  (params (Key :type Key%20Structure :default "None"))
  (:Pressed
    (if (Variables|/Game/FirstPerson/Blueprints/BP_FirstPersonCharacter.BP_FirstPersonCharacter_C|Getcone_collected (stale Collision|EventActorBeginOverlap _asbp_first_person_character))
      (bind _newtrack_1 (Timeline|Timeline Play)
        (:Update
          (Transformation|SetWorldLocation (Variables|Default|GetCube) (Math|Vector|Lerp(Vector) (Transformation|GetWorldLocation (Variables|Default|GetCube)) "0.000000,0.000000,300.000000" _newtrack_1) false false)))
      (else
        (Development|PrintString "can't move")))))

(fn ConstructionScript)