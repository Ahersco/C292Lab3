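; BP_TriggerZone is a trigger actor that lets the first-person player switch a referenced Light on and off while inside it.
; Entering hides the Light, sets the character's LightOff flag and enables input on the zone; leaving disables that input.
; The 1 key drives a FlipFlop that alternately shows and hides the Light, updating LightOff to match.
; Entry does not reset the FlipFlop.
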(event Collision|EventActorBeginOverlap
  (params (OtherActor :type Actor%20Object%20Reference))
  (bind _asbp_first_person_character (Utilities|Casting|CastToBP_FirstPersonCharacter OtherActor))
  (Variables|/Game/FirstPerson/Blueprints/BP_FirstPersonCharacter.BP_FirstPersonCharacter_C|SetLight_Off? _asbp_first_person_character true)
  (Rendering|SetActorHiddenInGame (Variables|Default|GetLight) true)
  (Input|EnableInput (Game|GetPlayerController 0)))

(event Collision|EventActorEndOverlap
  (params (OtherActor :type Actor%20Object%20Reference))
  (Utilities|Casting|CastToBP_FirstPersonCharacter OtherActor)
  (Input|DisableInput (Game|GetPlayerController 0)))

(event Input|KeyboardEvents|1
  (params (Key :type Key%20Structure :default "None"))
  (bind _light (Variables|Default|GetLight))
  (:Pressed
    (Utilities|FlowControl|FlipFlop
      (:A
        (Rendering|SetActorHiddenInGame _light false)
        (Variables|/Game/FirstPerson/Blueprints/BP_FirstPersonCharacter.BP_FirstPersonCharacter_C|SetLight_Off? (stale Collision|EventActorBeginOverlap _asbp_first_person_character) false))
      (:B
        (Rendering|SetActorHiddenInGame _light true)
        (Variables|/Game/FirstPerson/Blueprints/BP_FirstPersonCharacter.BP_FirstPersonCharacter_C|SetLight_Off? (stale Collision|EventActorBeginOverlap _asbp_first_person_character) true)))))

(fn ConstructionScript)